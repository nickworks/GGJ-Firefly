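; Firefly actor that blinks its glow and, while flagged as following, flies around the player pawn.
; Steering applies a clamped seek force toward the pawn's location plus a periodically rerolled random offset.
; A timer toggles glow randomly, or follows GlowPattern with pulse particles while Detector is overlapped and not following, easing the material's GlowStrength.
; Detector overlaps also enable or disable player input on the actor.
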(event OnComponentBeginOverlap(Detector)
  (params (OverlappedComponent :type Primitive%20Component%20Object%20Reference) (OtherActor :type Actor%20Object%20Reference) (OtherComp :type Primitive%20Component%20Object%20Reference) (OtherBodyIndex :type Integer) (bFromSweep :type Boolean) (SweepResult :type Hit%20Result%20Structure%20%28by%20ref%29))
  (Input|EnableInput (Game|GetPlayerController 0))
  (Variables|Default|SetdoingPattern true))

(event OnComponentEndOverlap(Detector)
  (params (OverlappedComponent :type Primitive%20Component%20Object%20Reference) (OtherActor :type Actor%20Object%20Reference) (OtherComp :type Primitive%20Component%20Object%20Reference) (OtherBodyIndex :type Integer))
  (Input|DisableInput (Game|GetPlayerController 0))
  (Variables|Default|SetdoingPattern false))

(event EventBeginPlay)

(event Collision|EventActorBeginOverlap
  (params (OtherActor :type Actor%20Object%20Reference)))

(event EventTick
  (params (DeltaSeconds :type Float%20%28single-precision%29))
  (CallFunction|SetGlowAmount)
  (if (Variables|Default|GetisFollowingPlayer)
    (CallFunction|UpdateTarget)
    (CallFunction|SteerTowardsTarget)))

(fn ConstructionScript)

(fn SteerTowardsTarget
  (Physics|AddForce (Variables|Default|GetSphere) (- (Math|Vector|ClampVectorSize (- (Variables|Default|GetTarget) (Transformation|GetActorLocation)) 0.0 (Variables|Default|GetMAX_SPEED)) (Transformation|GetVelocity)) "None" true))

(fn UpdateTarget
  (Utilities|IsValid (Variables|Default|GetTargetActor)
    (:Is%20Valid
      (bind _output_get (Variables|Default|SettimerUpdateTarget (- (Variables|Default|GettimerUpdateTarget) (Utilities|Time|GetWorldDeltaSeconds))))
      (if (<= _output_get 0.0)
        (CallFunction|RandomOffset)
        (Variables|Default|SettimerUpdateTarget (Math|Random|RandomFloatinRange 0.5 2.0)))
      (Variables|Default|SetTarget (+ (Transformation|GetActorLocation (Variables|Default|GetTargetActor)) (Variables|Default|Getoffset))))
    (:Is%20Not%20Valid
      (Variables|Default|SetTargetActor (Game|Player|GetPlayerPawn 0)))))

(fn RandomOffset
  (Variables|Default|Setoffset (* (Math|Random|RandomUnitVector) (Math|Random|RandomFloatinRange 5e+01 5e+02))))

(fn SetGlowAmount
  (bind _glowpattern (Variables|Default|GetglowPattern))
  (bind _returnvalue (Utilities|Array|Length _glowpattern))
  (Utilities|FlowControl|Sequence
    (:then_0
      ;[1 1 1] Fade using exponential slide
      (Variables|Default|SetglowAmount (+ (Variables|Default|GetglowAmount) (* (- (select (Variables|Default|GetisGlowing) (Math|Float|MakeLiteralFloat 1.0) (Math|Float|MakeLiteralFloat 0.0)) (Variables|Default|GetglowAmount)) (Utilities|Time|GetWorldDeltaSeconds) (Variables|Default|GetfadeEasing)))))
    (:then_1
      ;[1 1 1] Countdown the glow timer
      (bind _output_get (Variables|Default|SettimerUpdateGlow (- (Variables|Default|GettimerUpdateGlow) (Utilities|Time|GetWorldDeltaSeconds))))
      (if (<= _output_get 0.0)
        (Variables|Default|SetisGlowing (not (Variables|Default|GetisGlowing)))
        (if (or (Variables|Default|GetisFollowingPlayer) (not (Variables|Default|GetdoingPattern)))
          ;[1 1 1] Random blinking
          (Variables|Default|SettimerUpdateGlow (Math|Random|RandomFloatinRange 0.5 2.5))
          (else
            ;[1 1 1] Blink the pattern
            (if (> _returnvalue 0)
              (bind _output_get_2 (Variables|Default|SetpatternIndex (Math|Integer|%(Integer) (+ (Variables|Default|GetpatternIndex) 1) _returnvalue)))
              (Variables|Default|SettimerUpdateGlow (Utilities|Array|Get(acopy) (Variables|Default|GetglowPattern) _output_get_2))
              (if (Variables|Default|GetisGlowing)
                (Effects|SpawnEmitteratLocation "/Game/Effects/Pulse.Pulse" (Transformation|GetActorLocation) "0, 0, 0" "3.000000,3.000000,3.000000")))))))
    (:then_2
      ;[1 1 1] Update material
      (Rendering|Material|SetScalarParameterValueonMaterials (Variables|Default|GetStaticMesh) "GlowStrength" (Variables|Default|GetglowAmount)))))